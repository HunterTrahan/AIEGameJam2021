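; Knife-throw wheel actor that spins continuously at a rate set by WheelSpeed.
; Each Tick adds frame-time-scaled speed to WheelAngle and applies it as actor pitch, with yaw fixed at 90 and roll at zero.
; The angle resets to zero after reaching a full turn, discarding any overshoot.
; The Blueprint contains no knife, hit or overlap logic.
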(event `self.ReceiveTick`
  (params (DeltaSeconds :type "Float (single-precision)"))
  (set `self.Wheel Angle` (+ (* DeltaSeconds (`self.Wheel Speed`)) (`self.Wheel Angle`)))
  (`self.K2_SetActorRotation` (`KismetMathLibrary.MakeRotator` 0.0 (`self.Wheel Angle`) 90.0))
  (if (>= (`self.Wheel Angle`) 360.0)
    (set `self.Wheel Angle` 0.0)))

(fn `UserConstructionScript`)