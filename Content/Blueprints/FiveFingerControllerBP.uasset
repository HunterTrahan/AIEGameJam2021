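; Controller for a five-finger stab minigame, moving the player pawn between points on a hand under a dedicated camera.
; StartMinigame caches the hand's point locations; Tick steps the pawn toward its destination at fixed per-frame speed, returning via a halfway point.
; A random, left-biased mouse-button prompt shows in UIBP.
; Correct presses advance a forward-and-reverse stab sequence after a short delay; wrong ones reset it.
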(event `self.ReceiveBeginPlay`
  (bind _returnvalue (`|CreateWidget` "/Game/Blueprints/UIBP.UIBP_C"))
  (set `self.UI Widget` _returnvalue)
  (`UserWidget.AddToViewport` _returnvalue 0)
  (set `self.Current Destination` (`self.Point One`))
  (`self.Generate Correct Key`))

(event `self.ReceiveTick`
  (params (DeltaSeconds :type "Float (single-precision)"))
  (if (== (`self.Current Destination`) (`self.K2_GetActorLocation` (`GameplayStatics.GetPlayerPawn` 0)) :`ErrorTolerance` 2.0)
    (if (== (`self.Current Destination`) (`self.Return Halfway`) :`ErrorTolerance` 1.0)
      (set `self.Current Destination` (`self.Return Point`))
      (elif (!= (`self.Current Destination`) (`self.Return Point`))
        (set `self.Current Destination` (`self.Return Halfway`))))
    (else
      (`self.Move To Point` (`self.Current Destination`)))))

(event `Key|LeftMouseButton`
  (params (Key :type "Key Structure"))
  (:`Pressed`
    (if (== Key (`self.Correct Key`))
      (set `self.Current Destination` (`self.Return Halfway`) :!label _label)
      (`KismetSystemLibrary.Delay` 0.2)
      (switch `/Game/Blueprints/FiveFingerEnumBP` (`self.CurrentStab`)
        (:`NewEnumerator0`
          (set `self.Current Destination` (`self.Point Three`))
          (set `self.CurrentStab` "NewEnumerator1"))
        (:`NewEnumerator1`
          (set `self.Current Destination` (`self.Point Two`))
          (set `self.CurrentStab` "NewEnumerator2"))
        (:`NewEnumerator2`
          (set `self.Current Destination` (`self.Point One`))
          (set `self.CurrentStab` "NewEnumerator3"))
        (:`NewEnumerator3`
          (set `self.Current Destination` (`self.Point Two`))
          (set `self.CurrentStab` "NewEnumerator4"))
        (:`NewEnumerator4`
          (set `self.Current Destination` (`self.Point Three`))
          (set `self.CurrentStab` "NewEnumerator5")))
      (`self.Generate Correct Key`)
      (else
        (set `self.CurrentStab` "NewEnumerator0" :!label _label_2)))))

(event `Key|RightMouseButton`
  (params (Key :type "Key Structure"))
  (:`Pressed`
    (if (== Key (`self.Correct Key`))
      (goto _label)
      (else
        (goto _label_2)))))

(event `Generate Correct Key`
  (if (< (`KismetMathLibrary.RandomInteger` 3) 2)
    (set `self.Correct Key` "LeftMouseButton")
    (set `self.OutputText` "Left Mouse Button")
    (else
      (set `self.Correct Key` "RightMouseButton")
      (set `self.OutputText` "Right Mouse Button")))
  (`/Game/Blueprints/UIBP.Set Text` (`self.UI Widget`) (`self.OutputText`)))

(fn `End Minigame`
  (`self.K2_SetActorRotation` (`GameplayStatics.GetPlayerPawn` 0) (struct) false))

(fn `Move To Point`
  (params (Destination :type "Vector Structure"))
  (bind _returnvalue (`GameplayStatics.GetPlayerCharacter` 0))
  (bind _returnvalue_2 (`self.K2_GetActorLocation` _returnvalue))
  (`self.K2_SetActorLocation` _returnvalue (+ (* (`KismetMathLibrary.GetForwardVector` (`KismetMathLibrary.FindLookAtRotation` _returnvalue_2 Destination)) 3) _returnvalue_2) false false))

(fn `Start Minigame`
  (`self.K2_SetActorRotation` (`GameplayStatics.GetPlayerPawn` 0) (struct :`Pitch` -90.0) false)
  (set `self.Point One` (`SceneComponent.K2_GetComponentLocation` (`/Game/Blueprints/FiveFingerHand.Coordinate Point` (`self.Hand Component`))))
  (`self.SetViewTargetWithBlend` self (`self.FiveFingerCamera`) 0.0 "VTBlend_Linear" 0.0 false)
  (`self.K2_SetActorLocation` (`GameplayStatics.GetPlayerPawn` 0) (+ (`self.K2_GetActorLocation` (`self.Hand Component`)) (0.0 0.0 65.0)) false false)
  (set `self.Return Halfway` (`SceneComponent.K2_GetComponentLocation` (`/Game/Blueprints/FiveFingerHand.Return Half` (`self.Hand Component`))))
  (set `self.Return Point` (`SceneComponent.K2_GetComponentLocation` (`/Game/Blueprints/FiveFingerHand.Return Point` (`self.Hand Component`))))
  (set `self.Point Two` (`SceneComponent.K2_GetComponentLocation` (`/Game/Blueprints/FiveFingerHand.Coordinate Point1` (`self.Hand Component`))))
  (set `self.Point Three` (`SceneComponent.K2_GetComponentLocation` (`/Game/Blueprints/FiveFingerHand.Coordinate Point2` (`self.Hand Component`)))))

(fn `UserConstructionScript`)